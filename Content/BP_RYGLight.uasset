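; BP_RYGLight is a traffic light actor that cycles endlessly through red, green and yellow.
; From BeginPlay it calls TurnLight for each colour, waits for that colour's RTime, GTime or YTime delay, then loops through the ReStart event.
; TurnLight hides all three light components, shows the requested one and prints a debug message; its Time input is unused.
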(event `self.ReceiveBeginPlay`
  (`self.TurnLight` 0 "R" :!label _label)
  (`KismetSystemLibrary.Delay` (`KismetMathLibrary.Conv_IntToDouble` (`self.r_time`)))
  (`self.TurnLight` 0 "G")
  (`KismetSystemLibrary.Delay` (`KismetMathLibrary.Conv_IntToDouble` (`self.g_time`)))
  (`self.TurnLight` 0 "Y")
  (`KismetSystemLibrary.Delay` (`KismetMathLibrary.Conv_IntToDouble` (`self.y_time`)))
  (`self.ReStart`))

(event `ReStart`
  (goto _label))

(fn `TurnLight`
  (params (time :type Integer) (light :type String))
  (`SceneComponent.SetVisibility` (`self.light_G`) false false)
  (`SceneComponent.SetVisibility` (`self.light_R`) false false)
  (`SceneComponent.SetVisibility` (`self.light_Y`) false false)
  (switch `string` light
    (:`R`
      (`SceneComponent.SetVisibility` (`self.light_R`) true false)
      (`KismetSystemLibrary.PrintString` "R ON"))
    (:`Y`
      (`SceneComponent.SetVisibility` (`self.light_Y`) true false)
      (`KismetSystemLibrary.PrintString` "Y ON"))
    (:`G`
      (`SceneComponent.SetVisibility` (`self.light_G`) true false)
      (`KismetSystemLibrary.PrintString` "G ON"))))

(fn `UserConstructionScript`)